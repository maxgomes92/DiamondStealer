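; Stealth level logic that runs an emerald heist objective, from theft to evacuation.
; On BeginPlay it spawns the Emerald, binds to its pickup event, creates the player HUD with the steal objective and plays the theme music.
; Pickup changes the HUD objective to evacuation and plays the OpenGates level sequence.
; HandleGameOver shows the game over widget but is not called within this Blueprint.
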(event `EmeraldHasBeenPickedUp`
  (`self.HandleEmeraldHasBeenPickedup`))

(event `self.ReceiveBeginPlay`
  (bind _returnvalue (`|SpawnActorFromClass` "/Game/Blueprints/Emerald.Emerald_C" (`KismetMathLibrary.MakeTransform` (0.0 0.0 75.0)) "Undefined" "OverrideRootScale" null null))
  (add `/Game/Blueprints/Emerald.HasBeenPickedUp` _returnvalue (delegate `EmeraldHasBeenPickedUp`))
  (`self.SetupHUD`)
  (`GameplayStatics.PlaySound2D` "/Game/Sounds/stealth_theme.stealth_theme" 1.0 1.0 0.0 null null))

(fn `HandleEmeraldHasBeenPickedup`
  (`/Game/HUD/Player_HUD.UpdateHUD` (`self.PlayerHUDRef`) "Evacuate the area")
  (bind (_outactor _returnvalue) (`LevelSequencePlayer.CreateLevelSequencePlayer` "/Game/Sequencers/OpenGates.OpenGates"))
  (`MovieSceneSequencePlayer.Play` _returnvalue))

(fn `HandleGameOver`
  (bind _returnvalue (`|CreateWidget` "/Game/HUD/GameOver_HUD.GameOver_HUD_C"))
  (`UserWidget.AddToViewport` _returnvalue 0))

(fn `SetupHUD`
  (bind _returnvalue (`|CreateWidget` "/Game/HUD/Player_HUD.Player_HUD_C"))
  (bind _output_get (set `self.PlayerHUDRef` _returnvalue))
  (`/Game/HUD/Player_HUD.UpdateHUD` _output_get "Steal the emerald without getting caught")
  (`UserWidget.AddToViewport` _output_get 0))

(fn `UserConstructionScript`)