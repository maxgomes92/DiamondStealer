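; Behavior tree task that picks the world location of the current patrol point for an Enemy pawn.
; It reads the path index from the blackboard, takes that local point from the enemy's PatrolPath actor and transforms it into world space.
; The result is written to a blackboard vector key and the task succeeds; with no valid path or Enemy cast, it never finishes.
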(event `self.ReceiveExecuteAI`
  (params (OwnerController :type "AIController Object Reference") (ControlledPawn :type "Pawn Object Reference"))
  (bind _asenemy (cast `/Game/Blueprints/Enemy/Enemy` ControlledPawn))
  (bind _patrolpath (`/Game/Blueprints/Enemy/Enemy.PatrolPath` _asenemy)
    (:`then`
      (`BTFunctionLibrary.SetBlackboardValueAsVector` (`self.BB_Path`) (`KismetMathLibrary.TransformLocation` (`Actor.GetTransform` _patrolpath) (`|GetArrayItem` (`/Game/Blueprints/Enemy/PatrolPath.PathPoints` _patrolpath) (`BTFunctionLibrary.GetBlackboardValueAsInt` (`self.BB_PathIndex`)))))
      (`self.FinishExecute` true))
    (:`else`)))