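; Behavior tree task that advances an Enemy's patrol index to the next point on its patrol path.
; On AI execution it casts the controlled pawn to Enemy and reads the path index from the Blackboard.
; A math expression adds one and wraps by the PathPoints count, looping the patrol, then the task writes the index back and finishes successfully.
; A failed cast stops without finishing the task.
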(event EventReceiveExecuteAI
  (params (OwnerController :type AI%20Controller%20Object%20Reference) (ControlledPawn :type Pawn%20Object%20Reference))
  (bind _asenemy (Utilities|Casting|CastToEnemy ControlledPawn))
  (Class|BTFunctionLibrary|SetBlackboardValueasInt (Variables|Default|GetBB_PathIndex) (|((current+1)%lenth) (Class|BTFunctionLibrary|GetBlackboardValueasInt (Variables|Default|GetBB_PathIndex)) (Utilities|Array|Length (Variables|/Game/Blueprints/Enemy/PatrolPath.PatrolPath_C|GetPathPoints (Variables|/Game/Blueprints/Enemy/Enemy.Enemy_C|GetPatrolPath _asenemy)))))
  (AI|BehaviorTree|FinishExecute true))